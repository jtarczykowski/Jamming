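; Pickup-style interactable actor that a TopDownCharacter can carry and that returns to its starting spot when dropped.
; BecomeInteractitve briefly flashes a PaperSprite icon, which Tick holds at a fixed world rotation and scale.
; Interact passes the actor to the character's Pickup and queries TargetTag actors without using the result.
; Drop hides the icon, detaches, teleports to the position saved at BeginPlay, and calls an empty OnDropped hook.
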(event Custom|ShowIcon
  (bind _papersprite (Variables|Default|GetPaperSprite))
  (Development|SetHiddeninGame _papersprite false true)
  (Utilities|FlowControl|Delay 0.2)
  (Development|SetHiddeninGame _papersprite true true))

(event EventBecomeInteractitve
  (|CallParentFunction)
  (CallFunction|ShowIcon))

(event EventInteract
  (params (actor :type Actor%20Object%20Reference))
  ;[1 1 1] Interact
  (bind _astop_down_character (Utilities|Casting|CastToTopDownCharacter actor))
  (Default|Pickup _astop_down_character self)
  (Actor|GetAllActorswithTag (Variables|Default|GetTargetTag)))

(event EventBeginPlay
  (Variables|Default|SetOriginalPosition (Transformation|GetActorLocation)))

(event EventTick
  (params (DeltaSeconds :type Float%20%28single-precision%29))
  (bind _papersprite (Variables|Default|GetPaperSprite))
  (|CallParentFunction DeltaSeconds)
  (Transformation|SetWorldRotation _papersprite (Math|Rotator|MakeRotator 315.0 0.0 9e+01) false false)
  (Transformation|SetWorldScale3D _papersprite "0.200000,0.200000,0.200000"))

(event Custom|Drop
  (Development|SetHiddeninGame (Variables|Default|GetPaperSprite) true false)
  (Transformation|DetachFromActor "KeepWorld" "KeepWorld" "KeepWorld")
  (Transformation|SetActorLocation (Variables|Default|GetOriginalPosition) false true)
  (CallFunction|OnDropped))

(event Custom|OnDropped)

(fn ConstructionScript)