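; BP_Pralka is a washing machine (Polish "pralka") consumer that turns collected shirts ("koszule") into a spawned BP_Koszule.
; Each OnConsumed call from the parent increments a counter; once it reaches four, the Box collision is disabled and a progress-bar widget appears.
; A Timeline drives the bar, then spawns BP_Koszule at the machine's transform and hides the widget.
; The counter and collision are never reset here.
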(event EventBeginPlay
  (|CallParentFunction))

(event Collision|EventActorBeginOverlap
  (params (OtherActor :type Actor%20Object%20Reference)))

(event EventTick
  (params (DeltaSeconds :type Float%20%28single-precision%29)))

(event EventOnConsumed
  (|CallParentFunction)
  (bind _result (Math|Integer|IncrementInt (Variables|Default|GetConsumedKoszule))
    (:%20%20
      (if (>= _result 4)
        (Development|SetHiddeninGame (Variables|Default|GetWidget) false false)
        (Collision|SetCollisionEnabled (Variables|Default|GetBox) "NoCollision")
        (Components|Timeline|SetPlayRate (Variables|Default|GetTimeline_0) 1.0)
        (bind _percent (Timeline|Timeline_0 Play)
          (:Update
            (bind _asprogress_bar (Utilities|Casting|CastToProgressBar (UserInterface|GetUserWidgetObject (Variables|Default|GetWidget))))
            (Progress|SetPercent (Variables|/Game/BengHouse/UI/ProgressBar.ProgressBar_C|GetProgressBar_23 _asprogress_bar) _percent))
          (:Finished
            (Game|SpawnActorfromClass "/Game/BengHouse/Blueprints/Interaktable/BP_Koszule.BP_Koszule_C" (Transformation|GetActorTransform self) "Undefined" 0 0)
            (Development|SetHiddeninGame (Variables|Default|GetWidget) true false)))))))

(fn ConstructionScript
  (|CallParentFunction))