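; BP_Ksiazka is an interactable book actor, built as a child of a parent Blueprint that supplies Interact and OnDropped events.
; Interact runs the parent logic and then hides the Book component in game.
; OnDropped runs the parent logic and then makes the Book component visible again.
; BeginPlay, overlap and Tick are unused, and the construction script only calls its parent.
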(event EventBeginPlay
  (|CallParentFunction) ; This node is disabled and will not be called.\nDrag off pins to build functionality.
)

(event Collision|EventActorBeginOverlap
  (params (OtherActor :type Actor%20Object%20Reference)))

(event EventTick
  (params (DeltaSeconds :type Float%20%28single-precision%29)))

(event EventInteract
  (params (actor :type Actor%20Object%20Reference))
  (|CallParentFunction actor)
  (Development|SetHiddeninGame (Variables|Default|GetBook) true false))

(event EventOnDropped
  (|CallParentFunction)
  (Development|SetHiddeninGame (Variables|Default|GetBook) false false))

(fn ConstructionScript
  (|CallParentFunction))