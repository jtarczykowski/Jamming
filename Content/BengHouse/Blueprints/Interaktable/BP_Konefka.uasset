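; BP_Konefka is an interactable Blueprint, apparently a watering can by its name, that can be picked up and dropped.
; It extends the parent's Interact and OnDropped events, calling the parent logic first in each.
; Interact then disables collision on the Konefka component, and OnDropped restores it to query and physics.
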(event EventBeginPlay
  (|CallParentFunction) ; This node is disabled and will not be called.\nDrag off pins to build functionality.
)

(event Collision|EventActorBeginOverlap
  (params (OtherActor :type Actor%20Object%20Reference)))

(event EventTick
  (params (DeltaSeconds :type Float%20%28single-precision%29)))

(event EventInteract
  (params (actor :type Actor%20Object%20Reference))
  (|CallParentFunction actor)
  (Collision|SetCollisionEnabled (Variables|Default|GetKonefka) "NoCollision"))

(event EventOnDropped
  (|CallParentFunction)
  (Collision|SetCollisionEnabled (Variables|Default|GetKonefka) "QueryAndPhysics"))

(fn ConstructionScript
  (|CallParentFunction))