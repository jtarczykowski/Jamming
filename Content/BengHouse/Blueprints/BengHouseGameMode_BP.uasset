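; Game mode for BengHouse that runs the flow of a two-player round with a shared cumulative score.
; On BeginPlay it fades in gameplay music, shows the HUD and enables input for both players.
; EndGame swaps the HUD for a finishing widget and disables input, while AddPoints updates the total and notifies the HUD.
; A start-screen setup that also creates the second player is left unconnected.
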(event Custom|StartGame
  (bind _returnvalue (Game|GetPlayerController 0))
  (bind _returnvalue_2 (UserInterface|CreateWidget "/Game/BengHouse/UI/UI_HUD.UI_HUD_C" _returnvalue))
  (bind _output_get (Variables|Default|SetHUDWidget _returnvalue_2))
  (UserInterface|Viewport|AddtoViewport _output_get 0)
  (Input|EnableInput (Game|GetPlayerCharacter 0) _returnvalue)
  (Input|EnableInput (Game|GetPlayerCharacter 1) (Game|GetPlayerController 1)))

(event Custom|EndGame
  (Widget|RemovefromParent (Variables|Default|GetHUDWidget))
  (bind _returnvalue (UserInterface|CreateWidget "/Game/BengHouse/UI/FinishingWidget.FinishingWidget_C" (Game|GetPlayerController 0)))
  (UserInterface|Viewport|AddtoViewport _returnvalue 0)
  (Input|DisableInput (Game|GetPlayerCharacter 0) (Game|GetPlayerController 0))
  (Input|DisableInput (Game|GetPlayerCharacter 1) (Game|GetPlayerController 1)))

(event Custom|AddPoints
  (Variables|Default|SetCummulatedPoints (+ (Variables|Default|GetCummulatedPoints) (Variables|Default|GetAddedPoints)))
  (Default|AddPoints (Variables|/Game/BengHouse/UI/UI_HUD.UI_HUD_C|GetPoints (Variables|Default|GetHUDWidget))))

(event Custom|StartMusic
  (bind _returnvalue (Audio|SpawnSound2D "/Game/BengHouse/Sounds/Music/Mus_Gameplay_01.Mus_Gameplay_01" 1.0 1.0 0.0 0))
  (Audio|Components|Audio|FadeIn _returnvalue 6.0 1.0 0.0 :!class /Script/Engine.AudioComponent))

(event EventBeginPlay
  (bind _returnvalue (Game|GetPlayerController 0))
  (Utilities|FlowControl|Sequence
    (:then_0
      (bind _returnvalue_2 (Audio|SpawnSound2D "/Game/BengHouse/Sounds/Music/Mus_Gameplay_01.Mus_Gameplay_01" 1.0 1.0 0.0 0))
      (Audio|Components|Audio|FadeIn _returnvalue_2 6.0 1.0 0.0 :!class /Script/Engine.AudioComponent))
    (:then_1
      (bind _returnvalue_3 (UserInterface|CreateWidget "/Game/BengHouse/UI/UI_HUD.UI_HUD_C" _returnvalue))
      (bind _output_get (Variables|Default|SetHUDWidget _returnvalue_3))
      (UserInterface|Viewport|AddtoViewport _output_get 0)
      (Input|EnableInput (Game|GetPlayerCharacter 0) _returnvalue)
      (Input|EnableInput (Game|GetPlayerCharacter 1) (Game|GetPlayerController 1)))))

(fn ConstructionScript)