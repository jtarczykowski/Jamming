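; Oven Blueprint that cooks over time and produces a roasted turkey (BP_IndykUpieczony) once its inherited OnConsumed event fires.
; On consumption it calls the parent logic, disables the Box collision and reveals its widget.
; The Cooking timeline feeds the widget's progress bar and spawns the turkey at the oven's transform when finished.
; The StartCooking event is an empty stub.
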(event Custom|StartCooking)

(event EventOnConsumed
  (|CallParentFunction)
  (Collision|SetCollisionEnabled (Variables|Default|GetBox) "NoCollision")
  (Development|SetHiddeninGame (Variables|Default|GetWidget) false false)
  (bind _percent (Timeline|Cooking Play)
    (:Update
      (bind _asprogress_bar (Utilities|Casting|CastToProgressBar (UserInterface|GetUserWidgetObject (Variables|Default|GetWidget))))
      (Progress|SetPercent (Variables|/Game/BengHouse/UI/ProgressBar.ProgressBar_C|GetProgressBar_23 _asprogress_bar) _percent))
    (:Finished
      (Game|SpawnActorfromClass "/Game/BengHouse/Blueprints/Interaktable/BP_IndykUpieczony.BP_IndykUpieczony_C" (Transformation|GetActorTransform self) "Undefined" 0 0))))

(fn ConstructionScript
  (|CallParentFunction))